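; Clickable tentacle actor that the player damages by clicking it from close range, showing a hand cursor on hover.
; Each click within range of the player character lowers its health and sets a Hit flag.
; At zero health it sets Killed, decrements TentacleCount on the FirstPersonCharacter, then after a delay destroys itself and restores the default cursor.
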(event MouseInput|EventActorEndCursorOver
  ;[1 1 1] Mouse Over
  (Variables|/Script/Engine.PlayerController|SetCurrentMouseCursor (Game|GetPlayerController 0) "Default"))

(event MouseInput|EventActorBeginCursorOver
  ;[1 1 1] Mouse Over
  (Variables|/Script/Engine.PlayerController|SetCurrentMouseCursor (Game|GetPlayerController 0) "Hand"))

(event MouseInput|EventActorOnClicked
  (params (ButtonPressed :type Key%20Structure))
  (bind _returnvalue (Game|GetPlayerCharacter 0))
  ;[1 1 1] On Click
  (Math|Float|CompareFloat (Transformation|GetDistanceTo _returnvalue self) 7e+02
    (:<
      (Variables|Default|SettentacleHealth (- (Variables|Default|GettentacleHealth) 1))
      (Variables|Default|SetHit true)
      (if (== (Variables|Default|GettentacleHealth) 0)
        (Variables|Default|Setkilled true)
        (bind _asfirst_person_character (Utilities|Casting|CastToFirstPersonCharacter _returnvalue))
        (Variables|/Game/FirstPersonBP/Blueprints/FirstPersonCharacter.FirstPersonCharacter_C|SettentacleCount _asfirst_person_character (- (Variables|/Game/FirstPersonBP/Blueprints/FirstPersonCharacter.FirstPersonCharacter_C|GettentacleCount _asfirst_person_character) 1))
        (Utilities|FlowControl|Delay 3.0)
        (Actor|DestroyActor)
        ;[1 1 1] Mouse Over
        (Variables|/Script/Engine.PlayerController|SetCurrentMouseCursor (Game|GetPlayerController 0) "Default")))))

(fn ConstructionScript)